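; Treeline is an Arena scenery Blueprint that lines a spline with randomly chosen tree meshes.
; The construction script steps along the spline at Spacing intervals, adding an unrotated, unit-scale static mesh component at each point.
; A random switch picks the tree mesh; its sixth branch is unreachable.
; All branches share bark material and cull distance setup, but the second material slot targets only the first branch's component.
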(event EventBeginPlay)

(event Collision|EventActorBeginOverlap
  (params (OtherActor :type Actor%20Object%20Reference)))

(event EventTick
  (params (DeltaSeconds :type Float%20%28single-precision%29)))

(fn ConstructionScript
  (bind _splinecomponent (Variables|Default|GetSplineComponent))
  (bind _spacing (Variables|Default|GetSpacing))
  (for _index (range 0 (.ReturnValue (Math|Float|Division(WholeandRemainder) (Spline|GetSplineLength _splinecomponent) _spacing)))
    (switch int (Math|Random|RandomInteger 5)
      (:0
        (bind _returnvalue (AddComponent|AddStaticMeshComponent false (Math|Transform|MakeTransform (Spline|GetLocationatDistanceAlongSpline _splinecomponent (* _index _spacing) "Local"))))
        (Components|StaticMesh|SetStaticMesh _returnvalue "/Game/Vegetation/Meshes/Trees/SM_tree1.SM_tree1"))
      (:1
        (bind _returnvalue_2 (AddComponent|AddStaticMeshComponent false (Math|Transform|MakeTransform (Spline|GetLocationatDistanceAlongSpline _splinecomponent (* _index _spacing) "Local"))))
        (Components|StaticMesh|SetStaticMesh _returnvalue_2 "/Game/Vegetation/Meshes/Trees/SM_tree3.SM_tree3"))
      (:2
        (bind _returnvalue_3 (AddComponent|AddStaticMeshComponent false (Math|Transform|MakeTransform (Spline|GetLocationatDistanceAlongSpline _splinecomponent (* _index _spacing) "Local"))))
        (Components|StaticMesh|SetStaticMesh _returnvalue_3 "/Game/Vegetation/Meshes/Trees/SM_tree9.SM_tree9"))
      (:3
        (bind _returnvalue_4 (AddComponent|AddStaticMeshComponent false (Math|Transform|MakeTransform (Spline|GetLocationatDistanceAlongSpline _splinecomponent (* _index _spacing) "Local"))))
        (Components|StaticMesh|SetStaticMesh _returnvalue_4 "/Game/Vegetation/Meshes/Trees/SM_tree7.SM_tree7"))
      (:4
        (bind _returnvalue_5 (AddComponent|AddStaticMeshComponent false (Math|Transform|MakeTransform (Spline|GetLocationatDistanceAlongSpline _splinecomponent (* _index _spacing) "Local"))))
        (Components|StaticMesh|SetStaticMesh _returnvalue_5 "/Game/Vegetation/Meshes/Trees/SM_tree8.SM_tree8"))
      (:5
        (bind _returnvalue_6 (AddComponent|AddStaticMeshComponent false (Math|Transform|MakeTransform (Spline|GetLocationatDistanceAlongSpline _splinecomponent (* _index _spacing) "Local"))))
        (Components|StaticMesh|SetStaticMesh _returnvalue_6 "/Game/Vegetation/Meshes/Trees/SM_tree9.SM_tree9")))
    (Rendering|Material|SetMaterial _returnvalue 0 "/Game/Vegetation/Material/Child_Material/M_deciduousbark2_Inst.M_deciduousbark2_Inst")
    (Rendering|Material|SetMaterial _returnvalue 1 "/Game/Vegetation/Material/Child_Material/M_tree_pro_Inst.M_tree_pro_Inst")
    (Class|PrimitiveComponent|SetCullDistance _returnvalue 3e+04)))