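; Fence actor that lines a spline with repeated wooden fence meshes.
; The construction script divides spline length by Spacing and adds a scaled Fence5 mesh component at each step, with an oak material and a cull distance.
; Mesh rotation combines the FenceRotateAngle yaw with the root component's world rotation, so pieces do not follow the spline tangent.
; The event graph contains no active logic.
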(event EventBeginPlay)

(event Collision|EventActorBeginOverlap
  (params (OtherActor :type Actor%20Object%20Reference)))

(event EventTick
  (params (DeltaSeconds :type Float%20%28single-precision%29)))

(fn ConstructionScript
  (bind _splinecomponent (Variables|Default|GetSplineComponent))
  (bind _spacing (Variables|Default|GetSpacing))
  (for _index (range 0 (.ReturnValue (Math|Float|Division(WholeandRemainder) (Spline|GetSplineLength _splinecomponent) _spacing)))
    (bind _returnvalue (AddComponent|AddStaticMeshComponent false (Math|Transform|MakeTransform (Spline|GetLocationatDistanceAlongSpline _splinecomponent (* _index _spacing) "Local") (Math|Rotator|CombineRotators (Math|Rotator|MakeRotator 0.0 0.0 (Variables|Default|GetFenceRotateAngle)) (Transformation|GetWorldRotation (Variables|Default|GetRootSceneComponent))) "1.500000,1.500000,1.500000")))
    (Components|StaticMesh|SetStaticMesh _returnvalue "/Game/Arena/Meshes/Fence5.Fence5")
    (Rendering|Material|SetMaterial _returnvalue 0 "/Game/StarterContent/Materials/M_Wood_Oak.M_Wood_Oak")
    (Class|PrimitiveComponent|SetCullDistance _returnvalue 3e+04)))