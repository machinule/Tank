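; Bushline is a spline-driven scenery actor that lines a path in the arena with bushes.
; Its Construction Script steps along the spline by Spacing, adding a separate, uniformly scaled, unrotated Static Mesh Component at each point.
; An unseeded random pick chooses among four bush meshes, so the mix can change on each reconstruction.
; All branches share one tail that applies the bush material and cull distance; the event graph is unused.
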(event EventBeginPlay)

(event Collision|EventActorBeginOverlap
  (params (OtherActor :type Actor%20Object%20Reference)))

(event EventTick
  (params (DeltaSeconds :type Float%20%28single-precision%29)))

(fn ConstructionScript
  (bind _splinecomponent (Variables|Default|GetSplineComponent))
  (bind _spacing (Variables|Default|GetSpacing))
  (for _index (range 0 (.ReturnValue (Math|Float|Division(WholeandRemainder) (Spline|GetSplineLength _splinecomponent) _spacing)))
    (switch int (Math|Random|RandomInteger 4)
      (:0
        (bind _returnvalue (AddComponent|AddStaticMeshComponent false (Math|Transform|MakeTransform (Spline|GetLocationatDistanceAlongSpline _splinecomponent (* _index _spacing) "Local") "0, 0, 0" "5.000000,5.000000,5.000000")))
        (Components|StaticMesh|SetStaticMesh _returnvalue "/Game/Vegetation/Meshes/Bush/SM_bush1.SM_bush1"))
      (:1
        (bind _returnvalue_2 (AddComponent|AddStaticMeshComponent false (Math|Transform|MakeTransform (Spline|GetLocationatDistanceAlongSpline _splinecomponent (* _index _spacing) "Local") "0, 0, 0" "5.000000,5.000000,5.000000")))
        (Components|StaticMesh|SetStaticMesh _returnvalue_2 "/Game/Vegetation/Meshes/Bush/SM_bush3.SM_bush3"))
      (:2
        (bind _returnvalue_3 (AddComponent|AddStaticMeshComponent false (Math|Transform|MakeTransform (Spline|GetLocationatDistanceAlongSpline _splinecomponent (* _index _spacing) "Local") "0, 0, 0" "5.000000,5.000000,5.000000")))
        (Components|StaticMesh|SetStaticMesh _returnvalue_3 "/Game/Vegetation/Meshes/Bush/SM_bush4.SM_bush4"))
      (:3
        (bind _returnvalue_4 (AddComponent|AddStaticMeshComponent false (Math|Transform|MakeTransform (Spline|GetLocationatDistanceAlongSpline _splinecomponent (* _index _spacing) "Local") "0, 0, 0" "5.000000,5.000000,5.000000")))
        (Components|StaticMesh|SetStaticMesh _returnvalue_4 "/Game/Vegetation/Meshes/Bush/SM_bush6.SM_bush6")))
    (Rendering|Material|SetMaterial _returnvalue 0 "/Game/Vegetation/Material/Child_Material/M_bush_pro_Inst.M_bush_pro_Inst")
    (Rendering|Material|SetMaterial _returnvalue 1 "/Game/Vegetation/Material/Child_Material/M_bush_pro_Inst.M_bush_pro_Inst")
    (Class|PrimitiveComponent|SetCullDistance _returnvalue 3e+04)))