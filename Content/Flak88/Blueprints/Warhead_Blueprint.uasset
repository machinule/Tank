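; Flak 88 warhead projectile that launches with a blast sound and emitter, then explodes on whatever it hits.
; BeginPlay adds a velocity of Speed along the actor's local Z to the physics root.
; Each Tick line-traces one frame of velocity ahead, catching impacts without relying on overlap events.
; A hit stops physics, snaps to the impact point, fires RadialForce, spawns larger effects, toggles visibility and destroys the actor after a delay.
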(event Collision|EventActorBeginOverlap
  (params (OtherActor :type Actor%20Object%20Reference)))

(event EventTick
  (params (DeltaSeconds :type Float%20%28single-precision%29))
  (bind _returnvalue (VehicleSound|GetRootComponent))
  (bind _radialforce (Variables|Default|GetRadialForce))
  (bind _returnvalue_2 (Transformation|GetWorldLocation _returnvalue))
  (bind (_outhit _returnvalue_3) (Collision|LineTraceByChannel _returnvalue_2 (+ _returnvalue_2 (* (Transformation|GetVelocity) DeltaSeconds)) "TraceTypeQuery1" false 0 "None"))
  (if _returnvalue_3
    (bind _asprimitive_component (Utilities|Casting|CastToPrimitiveComponent (VehicleSound|GetRootComponent)))
    (Physics|SetSimulatePhysics _asprimitive_component false)
    (Utilities|FlowControl|Sequence
      (:then_0
        (Transformation|SetActorLocation (.ImpactPoint (Collision|BreakHitResult _outhit)) false true)
        (Components|Activation|Activate _radialforce false))
      (:then_1
        (Class|RadialForceComponent|FireImpulse _radialforce)
        (bind _returnvalue_4 (Effects|SpawnEmitteratLocation "/Game/Flak88/Particles/P_Explosion.P_Explosion" (.ImpactPoint (Collision|BreakHitResult _outhit))))
        (Transformation|SetRelativeScale3D _returnvalue_4 "10.000000,10.000000,10.000000")
        (Audio|PlaySoundatLocation "/Game/Flak88/Audio/Explosion01.Explosion01" (.ImpactPoint (Collision|BreakHitResult _outhit)) "0, 0, 0" 2.0)
        (Rendering|ToggleVisibility (VehicleSound|GetRootComponent) false)
        (Utilities|FlowControl|Delay 5.0)
        (Actor|DestroyActor)))))

(event EventBeginPlay
  (bind _returnvalue (Transformation|GetActorLocation))
  (bind _asprimitive_component (Utilities|Casting|CastToPrimitiveComponent (VehicleSound|GetRootComponent)))
  (Physics|SetPhysicsLinearVelocity _asprimitive_component (Math|Vector|RotateVector (Math|Vector|MakeVector 0.0 0.0 (Variables|Default|GetSpeed)) (Transformation|GetActorRotation)) true "None")
  (Audio|PlaySoundatLocation "/Game/Flak88/Audio/Explosion01.Explosion01" _returnvalue)
  (bind _returnvalue_2 (Effects|SpawnEmitteratLocation "/Game/Flak88/Particles/P_Explosion.P_Explosion" _returnvalue))
  (Transformation|SetRelativeScale3D _returnvalue_2 "4.000000,4.000000,4.000000"))

(fn ConstructionScript)