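; Grabbable shell for the Flak 88 gun that loads when brought to the breech.
; Overlapping a "Loading"-tagged actor attached to a Flak88 that is ready to load drops the shell from the Grabber and passes it to LoadShell.
; LoadAnim plays the slide sound, moves the shell by accumulating local offsets from a timeline, then toggles the gun's breech when finished.
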(event EventBeginPlay
  (Input|EnableInput (Game|GetPlayerController 0)))

(event Collision|EventActorBeginOverlap
  (params (OtherActor :type Actor%20Object%20Reference))
  (bind _asflak_88 (Utilities|Casting|CastToFlak88 (Components|GetOwner (Transformation|GetAttachParent (VehicleSound|GetRootComponent OtherActor)))))
  (Variables|Default|SetFlak88 _asflak_88)
  (bind _returnvalue (Class|Flak88|ReadytoLoad _asflak_88))
  (if (and _returnvalue (Actor|ActorHasTag OtherActor "Loading"))
    (Class|TankCharacter|DropGrabbable (Variables|Default|GetGrabber))
    (Class|Flak88|LoadShell (Variables|Default|GetFlak88) self)))

(event EventTick
  (params (DeltaSeconds :type Float%20%28single-precision%29)))

(event EventLoadAnim
  (Audio|SpawnSoundatLocation "/Game/Flak88/Audio/ShellSlideBreech.ShellSlideBreech" (Transformation|GetWorldLocation (VehicleSound|GetRootComponent)))
  (bind _location (Timeline|Loading Play)
    (:Update
      (Transformation|AddActorLocalOffset _location false false))
    (:Finished
      (Class|Flak88|ToggleBreech (Variables|Default|GetFlak88)))))

(fn ConstructionScript)