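; Flak 88 gun Blueprint that provides firing and breech sound events, with no calls to them inside its own graph.
; BreechNoise and ShellSlideNoise play breech-closing and shell-slide sounds at the breech and loading sockets of the skeletal mesh.
; FireShell spawns a canister at the loading socket, calls DetachFromActor on itself, then spawns a warhead at the firing socket, each using its socket's rotation.
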(event Custom|ShellSlideNoise
  (bind _returnvalue (Audio|SpawnSoundatLocation "/Game/Flak88/Audio/ShellSlideBreech.ShellSlideBreech" (Transformation|GetSocketLocation (Class|SkeletalMesh|FindSocket (Variables|/Script/Engine.SkinnedMeshComponent|GetSkeletalMesh (Variables|Default|GetSkeletalMeshComponent)) "LoadingSocket") 0) "0, 0, 0" 0.25)))

(event EventBeginPlay)

(event Collision|EventActorBeginOverlap
  (params (OtherActor :type Actor%20Object%20Reference)))

(event EventFireShell
  (bind _returnvalue (VehicleSound|GetRootComponent))
  (bind _returnvalue_2 (VehicleSound|GetRootComponent))
  (Game|SpawnActorfromClass "/Game/Flak88/Blueprints/Canister_Blueprint.Canister_Blueprint_C" (Math|Transform|MakeTransform (Transformation|GetSocketLocation _returnvalue "LoadingSocket") (Math|Rotator|CombineRotators (Transformation|GetSocketRotation _returnvalue "LoadingSocket") "0.000000, 0, 0")) "AlwaysSpawn" 0 0)
  (Transformation|DetachFromActor "KeepRelative" "KeepRelative" "KeepRelative")
  (Game|SpawnActorfromClass "/Game/Flak88/Blueprints/Warhead_Blueprint.Warhead_Blueprint_C" (Math|Transform|MakeTransform (Transformation|GetSocketLocation _returnvalue_2 "FiringSocket") (Math|Rotator|CombineRotators (Transformation|GetSocketRotation _returnvalue_2 "FiringSocket") "0.000000, 0, 0")) "AlwaysSpawn" 0 0))

(event EventTick
  (params (DeltaSeconds :type Float%20%28single-precision%29)))

(event EventBreechNoise
  (bind _returnvalue (Audio|SpawnSoundatLocation "/Game/Flak88/Audio/BreechClosing.BreechClosing" (Transformation|GetSocketLocation (Class|SkeletalMesh|FindSocket (Variables|/Script/Engine.SkinnedMeshComponent|GetSkeletalMesh (Variables|Default|GetSkeletalMeshComponent)) "BreechSocket") 0) "0, 0, 0" 0.5)))

(fn ConstructionScript)